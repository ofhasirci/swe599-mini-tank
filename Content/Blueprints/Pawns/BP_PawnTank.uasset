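; BP_PawnTank is a tank pawn Blueprint that shows its health on a health bar widget.
; On BeginPlay it casts the HealthBar component's widget to WBP_HealthBar, caches it, sets the initial health and tints the progress bar blue.
; Tick then polls the health component and pushes the current value to the bar every frame, with no change events involved.
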(event EventBeginPlay
  (bind _aswbp_health_bar (Utilities|Casting|CastToWBP_HealthBar (UserInterface|GetUserWidgetObject (Variables|Default|GetHealthBar))))
  (bind _output_get (Variables|Default|SetHealtBarRef _aswbp_health_bar))
  (Default|UpdateHealth _output_get (Variables|/Script/ToonTanks.HealthComponent|GetHealth (Variables|Default|GetHealthCompnent)))
  (Class|ProgressBar|SetFillColorandOpacity (Variables|/Game/Blueprints/Widgets/WBP_HealthBar.WBP_HealthBar_C|GetProgress_Bar _output_get) "(R=0.088656,G=0.630757,B=0.879622,A=1.000000)"))

(event Collision|EventActorBeginOverlap
  (params (OtherActor :type Actor%20Object%20Reference)))

(event EventTick
  (params (DeltaSeconds :type Float%20%28single-precision%29))
  (Default|UpdateHealth (Variables|Default|GetHealtBarRef) (Variables|/Script/ToonTanks.HealthComponent|GetHealth (Variables|Default|GetHealthCompnent))))

(fn ConstructionScript)